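; Vase pickup that can be carried on a skeletal mesh and dropped back into the world.
; Pickup snaps it to the passed mesh's left wrist socket, disables collision on the DinoSaurRawr component and prints a debug message that labels it "Key".
; Drop detaches the actor in world space, then restores collision and turns on physics simulation for that component.
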(event `self.Pickup`
  (params (SkeletalMesh :type "SkeletalMeshComponent Object Reference"))
  (`KismetSystemLibrary.PrintText` (`|FormatText` "{Name} is up and attached to {mesh}" "Key" SkeletalMesh) true true (struct :`R` 0.049422 :`G` 1.0 :`A` 1.0))
  (`self.K2_AttachToComponent` SkeletalMesh "wrist_outer_l" "SnapToTarget" "SnapToTarget" "KeepRelative")
  (`PrimitiveComponent.SetCollisionEnabled` (`self.DinoSaurRawr`) "NoCollision"))

(event `self.Drop`
  (bind _dinosaurrawr (`self.DinoSaurRawr`))
  (`self.K2_DetachFromActor` "KeepWorld" "KeepWorld" "KeepWorld")
  (`PrimitiveComponent.SetCollisionEnabled` _dinosaurrawr "QueryAndPhysics")
  (`PrimitiveComponent.SetSimulatePhysics` _dinosaurrawr true))

(fn `UserConstructionScript`)