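; Dinosaur pickup actor that can be carried and dropped, with its dropped position recorded for saving.
; Pickup snaps it to the wrist_outer_l socket of the supplied skeletal mesh and disables collision.
; Drop detaches it, enables physics, and adds itself and the mesh's relative location to GM_SaveLoad's level-state arrays.
; NewDinoLocal moves the mesh to a supplied relative location.
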(event `/Game/Blueprints/Coding2Blueprints/BPI_Item.Pickup`
  (params (SkeletalMesh :type "SkeletalMeshComponent Object Reference"))
  (`KismetSystemLibrary.PrintText` (`|FormatText` "{Name} is up and attached to {mesh}" "Key" SkeletalMesh) true true (struct :`R` 0.049422 :`G` 1.0 :`A` 1.0))
  (`self.K2_AttachToComponent` SkeletalMesh "wrist_outer_l" "SnapToTarget" "SnapToTarget" "KeepRelative")
  (`PrimitiveComponent.SetCollisionEnabled` (`self.DinoSaurRawr`) "NoCollision"))

(event `/Game/Blueprints/Coding2Blueprints/BPI_Item.Drop`
  (bind _dinosaurrawr (`self.DinoSaurRawr`))
  (`self.K2_DetachFromActor` "KeepWorld" "KeepWorld" "KeepWorld")
  (`PrimitiveComponent.SetCollisionEnabled` _dinosaurrawr "QueryAndPhysics")
  (`PrimitiveComponent.SetSimulatePhysics` _dinosaurrawr true)
  (set `self.DinoLocals` (`SceneComponent.RelativeLocation` (`self.DinoSaurRawr`)))
  (bind _asgm_save_load (cast `/Game/Blueprints/Coding2Blueprints/SavingLoading/GM_SaveLoad` (`GameplayStatics.GetGameMode`)))
  (`KismetArrayLibrary.Array_AddUnique` (`/Game/Blueprints/Coding2Blueprints/SavingLoading/SG_LevelStates.DinoSaurs` (`/Game/Blueprints/Coding2Blueprints/SavingLoading/GM_SaveLoad.SG_LevelStates` _asgm_save_load)) self)
  (`KismetArrayLibrary.Array_AddUnique` (`/Game/Blueprints/Coding2Blueprints/SavingLoading/SG_LevelStates.DinoLocals` (`/Game/Blueprints/Coding2Blueprints/SavingLoading/GM_SaveLoad.SG_LevelStates` _asgm_save_load)) (`self.DinoLocals`)))

(event `NewDinoLocal`
  (params (DinoLocal :type "Vector Structure"))
  (`SceneComponent.K2_SetRelativeLocation` (`self.DinoSaurRawr`) DinoLocal false false))

(fn `UserConstructionScript`)