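; Exit actor that ends the game once two valuables are delivered into its trigger box.
; Overlaps from actors tagged RawrXD increment a counter shown as X/2 on a text render.
; At two, it shows the WBP_Ending widget with UI-only input and mouse cursor, then a timeline lowers the door cube.
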(event `self.Box.OnComponentBeginOverlap`
  (params (OverlappedComponent :type "PrimitiveComponent Object Reference") (OtherActor :type "Actor Object Reference") (OtherComp :type "PrimitiveComponent Object Reference") (OtherBodyIndex :type Integer) (bFromSweep :type Boolean) (SweepResult :type "HitResult Structure (by ref)"))
  (bind _returnvalue (`GameplayStatics.GetPlayerController` 0))
  (if (`self.ActorHasTag` OtherActor "RawrXD")
    (bind _result (`/Engine/EditorBlueprintResources/StandardMacros.IncrementInt` (`self.Valuables`))
      (:`  `
        (`TextRenderComponent.K2_SetText` (`self.TextRender`) (`|FormatText` "{int}/2" (`self.Valuables`)))
        (if (== _result 2)
          (bind _returnvalue_2 (`|CreateWidget` "/Game/WidgetsUI/WBP_Ending.WBP_Ending_C"))
          (`UserWidget.AddToViewport` _returnvalue_2 0)
          (`WidgetBlueprintLibrary.SetInputMode_UIOnlyEx` _returnvalue _returnvalue_2)
          (set `PlayerController.bShowMouseCursor` true _returnvalue)
          (bind (_direction _newtrack_0) (`Timeline|DoorOpensd`)
            (:`Update`
              (`SceneComponent.K2_SetRelativeLocation` (`self.Cube`) (`KismetMathLibrary.MakeVector` 0.0 0.0 (`KismetMathLibrary.Lerp` 140.0 -130.0 _newtrack_0)) false false))))))))

(fn `UserConstructionScript`)