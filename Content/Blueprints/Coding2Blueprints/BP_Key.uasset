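; BP_Key is a key item that can be picked up, dropped and used, with rotating movement while in the world.
; Pickup snaps it to the left wrist socket of the given skeletal mesh, disables collision, increments the player character's KeyTotal and stops rotation.
; Drop detaches it and enables collision and physics, leaving KeyTotal unchanged.
; UsePrimary is only a debug print.
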(event `self.ReceiveBeginPlay`
  (`KismetSystemLibrary.PrintString` "Key Exist" true true (struct :`R` 0.229185 :`G` 1.0 :`A` 1.0)))

(event `/Game/Blueprints/Coding2Blueprints/BPI_Item.Pickup`
  (params (SkeletalMesh :type "SkeletalMeshComponent Object Reference"))
  (`KismetSystemLibrary.PrintText` (`|FormatText` "{Name} is up and attached to {mesh}" "Key" SkeletalMesh) true true (struct :`R` 0.049422 :`G` 1.0 :`A` 1.0))
  (`self.K2_AttachToComponent` SkeletalMesh "wrist_outer_l" "SnapToTarget" "SnapToTarget" "KeepRelative")
  (`PrimitiveComponent.SetCollisionEnabled` (`self.StaticMesh`) "NoCollision")
  (bind _asbp_third_person_character (cast `/Game/ThirdPerson/Blueprints/BP_ThirdPersonCharacter` (`GameplayStatics.GetPlayerPawn` 0))
    (:`then`
      (bind _keytotal (`/Game/ThirdPerson/Blueprints/BP_ThirdPersonCharacter.KeyTotal` _asbp_third_person_character))
      (`/Engine/EditorBlueprintResources/StandardMacros.IncrementInt` _keytotal
        (:`  `
          (`KismetSystemLibrary.PrintString` (`KismetStringLibrary.Concat_StrStr` "Player now has " (`KismetStringLibrary.Conv_IntToString` _keytotal) " keys") true true (struct :`R` 0.229185 :`G` 1.0 :`A` 1.0))
          (`ActorComponent.Deactivate` (`self.RotatingMovement`)))))
    (:`CastFailed`
      (`KismetSystemLibrary.PrintString` "cast failed"))))

(event `/Game/Blueprints/Coding2Blueprints/BPI_Item.Drop`
  (`self.K2_DetachFromActor` "KeepWorld" "KeepWorld" "KeepWorld")
  (`PrimitiveComponent.SetCollisionEnabled` (`self.StaticMesh`) "QueryAndPhysics")
  (`PrimitiveComponent.SetSimulatePhysics` (`self.StaticMesh`) true))

(event `/Game/Blueprints/Coding2Blueprints/BPI_Item.UsePrimary`
  (`KismetSystemLibrary.PrintText` "USE KEY"))

(fn `UserConstructionScript`)