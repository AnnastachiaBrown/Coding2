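; Enemy spawner that populates the level with randomized BP_AiMoveTo characters when play begins.
; It finds every BP_EnemySpawnPoint and, with a 75% chance at each, spawns an enemy at that point's transform.
; Each spawned enemy gets a random name text, flat-color material and skeletal mesh from hardcoded arrays.
; A disconnected dynamic-material snippet for tinting remains unused.
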(event `self.ReceiveBeginPlay`
  (set `self.Array` (`|MakeArray` "Tommy" "Joe" "Bob" "Billy" "Jimmothy" :!type "Text"))
  (set `self.Array_0` (`|MakeArray` "/Game/Materials/MI_FlatYellow.MI_FlatYellow" "/Game/Materials/MI_FlatBlue.MI_FlatBlue" "/Game/Materials/MI_FlatRed.MI_FlatRed" "/Game/Materials/MI_FlatPink.MI_FlatPink" :!type "MaterialInterface Object Reference"))
  (set `self.Array_1` (`|MakeArray` "/Game/Characters/Mannequins/Meshes/SKM_Quinn.SKM_Quinn" "/Game/PolygonStarter/Models/Vehicles/SK_PolygonCity_Veh_Car_Small_01.SK_PolygonCity_Veh_Car_Small_01" "/Game/SCK_Casual01/Models/MESH_L_00.MESH_L_00" "/Game/PolygonStarter/Models/Characters/SK_Chr_Female_Face_01.SK_Chr_Female_Face_01" "/Game/Characters/Mannequin_UE4/Meshes/SK_Mannequin.SK_Mannequin" :!type "SkeletalMesh Object Reference"))
  (`KismetSystemLibrary.PrintString` "EnemySpawn Active" true true (struct :`R` 1.0 :`G` 0.094447 :`A` 1.0))
  (bind _outactors (`GameplayStatics.GetAllActorsOfClass` "/Game/Blueprints/Coding2Blueprints/BP_EnemySpawnPoint.BP_EnemySpawnPoint_C"))
  (for _array_element _outactors
    (if (`KismetMathLibrary.RandomBoolWithWeight` 0.75)
      (bind _returnvalue (`|SpawnActorFromClass` "/Game/AI_Blueprints/BP_AiMoveTo.BP_AiMoveTo_C" (`self.GetTransform` _array_element) "Undefined" "MultiplyWithRoot" null null))
      (`TextRenderComponent.K2_SetText` (`/Game/AI_Blueprints/BP_AiMoveTo.AINAme` _returnvalue) (`KismetArrayLibrary.Array_Random` (`self.Array`)))
      (`PrimitiveComponent.SetMaterial` (`Character.Mesh` _returnvalue) 0 (`KismetArrayLibrary.Array_Random` (`self.Array_0`)))
      (`SkeletalMeshComponent.SetSkeletalMeshAsset` (`Character.Mesh` _returnvalue) (`KismetArrayLibrary.Array_Random` (`self.Array_1`))))))

(fn `UserConstructionScript`)