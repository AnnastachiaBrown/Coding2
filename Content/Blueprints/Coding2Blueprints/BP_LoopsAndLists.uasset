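; BP_LoopsAndLists is a test Blueprint demonstrating loops and array operations through on-screen debug prints.
; BeginPlay starts DelayLoop, an endless self-calling event that increments and prints a counter, calls ColorPrint, then waits a second.
; ColorPrint loops once per ColorArray entry, printing random picks as colored text, then shuffles the array.
; BeginPlay sets ColorArray only after starting the loop, so the first pass runs before that assignment.
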(event `self.ReceiveBeginPlay`
  (`KismetSystemLibrary.PrintString` "Loops and List Active" true true (struct :`R` 1.0 :`G` 0.773418 :`A` 1.0))
  (`self.Delay Loop`)
  (set `self.ColorArray` (`|MakeArray` (struct :`R` 0.5 :`B` 0.055785 :`A` 1.0) (struct :`G` 0.5 :`A` 1.0) (struct :`B` 0.5 :`A` 1.0) (struct :`R` 0.521708 :`G` 0.57913 :`B` 0.075539 :`A` 1.0) :!type "LinearColor Structure")))

(event `Delay Loop`
  (bind _loopcount (`self.LoopCount`))
  (`KismetSystemLibrary.PrintString` "Starting Delay Loop " false true (struct :`R` 0.229185 :`G` 1.0 :`A` 1.0) 0.4)
  (`/Engine/EditorBlueprintResources/StandardMacros.IncrementInt` _loopcount
    (:`  `
      (`KismetSystemLibrary.PrintString` (`KismetStringLibrary.Concat_StrStr` "Loop #" (`KismetStringLibrary.Conv_IntToString` _loopcount)) false true (struct :`G` 0.66 :`B` 1.0 :`A` 1.0) 0.9)
      (`self.ColorPrint`)
      (`KismetSystemLibrary.Delay` 1.0)
      (`self.Delay Loop`))))

(event `ColorPrint`
  (bind _colorarray (`self.ColorArray`))
  (bind (_outitem _outindex) (`KismetArrayLibrary.Array_Random` _colorarray))
  (for _ _colorarray
    (`KismetSystemLibrary.PrintString` (`KismetStringLibrary.Concat_StrStr` "Printing Color #" (`KismetStringLibrary.Conv_IntToString` _outindex)) false true _outitem 0.9))
  (`KismetSystemLibrary.PrintString` "Color Done" false true (struct :`R` 0.229185 :`G` 1.0 :`A` 1.0))
  (`KismetArrayLibrary.Array_Shuffle` (`self.ColorArray`)))

(fn `UserConstructionScript`)