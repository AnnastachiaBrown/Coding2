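; BP_ItemSpawner populates the level with AI actors, acting as an enemy spawner despite its name.
; On BeginPlay it prints a debug message, finds every BP_ItemSpawnPoint, and gives each a weighted random chance to spawn a BP_AiMoveTo at that point's transform.
; An unfinished enemy material randomization, using a dynamic instance of MI_FlatRed, is left unconnected and never runs.
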(event `self.ReceiveBeginPlay`
  (`KismetSystemLibrary.PrintString` "EnemySpawn Active" true true (struct :`R` 1.0 :`G` 0.094447 :`A` 1.0))
  (bind _outactors (`GameplayStatics.GetAllActorsOfClass` "/Game/Blueprints/Coding2Blueprints/BP_ItemSpawnPoint.BP_ItemSpawnPoint_C"))
  (for _array_element _outactors
    (if (`KismetMathLibrary.RandomBoolWithWeight` 0.75)
      (`|SpawnActorFromClass` "/Game/AI_Blueprints/BP_AiMoveTo.BP_AiMoveTo_C" (`self.GetTransform` _array_element) "Undefined" "MultiplyWithRoot" null null))))

(fn `UserConstructionScript`)