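; Machine gun weapon that a character can pick up, use and drop, with firing and reloading stubbed as debug text.
; Pickup snaps it to the given skeletal mesh's hand_r socket and turns off body collision.
; Drop detaches it in world space, then restores collision and enables physics simulation on the body.
; Primary and secondary use only print placeholder fire and reload messages.
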(event `/Game/Blueprints/Coding2Blueprints/BPI_Item.Pickup`
  (params (SkeletalMesh :type "SkeletalMeshComponent Object Reference"))
  (`KismetSystemLibrary.PrintText` (`|FormatText` "{Name} is up and attached to {mesh}" "machine Gun" SkeletalMesh) true true (struct :`R` 0.049422 :`G` 1.0 :`A` 1.0))
  (`self.K2_AttachToComponent` SkeletalMesh "hand_r" "SnapToTarget" "SnapToTarget" "KeepRelative")
  (`PrimitiveComponent.SetCollisionEnabled` (`self.MachineGunBody`) "NoCollision"))

(event `/Game/Blueprints/Coding2Blueprints/BPI_Item.UsePrimary`
  (`KismetSystemLibrary.PrintText` "PEW PEW" true true (struct :`R` 1.0 :`A` 1.0)))

(event `/Game/Blueprints/Coding2Blueprints/BPI_Item.Drop`
  (bind _machinegunbody (`self.MachineGunBody`))
  (`self.K2_DetachFromActor` "KeepWorld" "KeepWorld" "KeepWorld")
  (`PrimitiveComponent.SetCollisionEnabled` _machinegunbody "QueryAndPhysics")
  (`PrimitiveComponent.SetSimulatePhysics` _machinegunbody true))

(event `/Game/Blueprints/Coding2Blueprints/BPI_Item.UseSecondary`
  (`KismetSystemLibrary.PrintText` "Reload"))

(fn `UserConstructionScript`)