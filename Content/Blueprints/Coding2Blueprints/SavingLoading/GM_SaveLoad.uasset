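; Game mode that saves and loads player stats and per-level progress, loading both on BeginPlay or creating new save objects when none exist.
; Player stats use a fixed slot and restore Stamina, Health and Mana on the third-person character.
; Level state uses a slot named after the current level, re-marking collected coins and opened key doors.
; Camera doors are iterated without effect, and level saves always report success.
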(event `self.ReceiveBeginPlay`
  (`KismetSystemLibrary.PrintString` "Loading the SaveLoad Game Mode" true true (struct :`R` 1.0 :`B` 0.406974 :`A` 1.0) 5.0)
  (`self.LoadPlayerStats`)
  (`self.LoadLevelState`))

(event `LoadPlayerStats`
  (bind _returnvalue (`GameplayStatics.DoesSaveGameExist` "PlayerSave")) ; Slot Name is the save file name
  (if _returnvalue
    (bind _returnvalue_2 (`GameplayStatics.LoadGameFromSlot` "PlayerSave")) ; slot name needs to be the same - copy and paste good
    (bind _assg_player_stats (cast `/Game/Blueprints/Coding2Blueprints/SavingLoading/SG_PlayerStats` _returnvalue_2))
    (bind _output_get (set `self.SG_PlayerStats` _assg_player_stats))
    (`self.UpdatePlayerInfo1` _output_get)
    (`KismetSystemLibrary.PrintString` "PlayerStats have been loaded" true true (struct :`R` 0.657476 :`G` 1.0 :`A` 1.0))
    (else
      (bind _returnvalue_3 (`GameplayStatics.CreateSaveGameObject` "/Game/Blueprints/Coding2Blueprints/SavingLoading/SG_PlayerStats.SG_PlayerStats_C"))
      (set `self.SG_PlayerStats` _returnvalue_3) ; set this variable so that the player\ncan edit these variables
    )))

(event `SavePlayerStats`
  (bind _returnvalue (`GameplayStatics.SaveGameToSlot` (`self.SG_PlayerStats`) "PlayerSave"))
  (if _returnvalue
    (`KismetSystemLibrary.PrintText` "PlayerStats Saved to save game file" true true (struct :`R` 0.06892 :`G` 1.0 :`A` 1.0) 5.0)
    (else
      (`KismetSystemLibrary.PrintText` "PlayerStats FAILED TO SAVE" true true (struct :`R` 1.0 :`B` 0.001431 :`A` 1.0) 5.0))))

(event `SaveLevelState`
  (bind _returnvalue (`GameplayStatics.GetCurrentLevelName` true))
  (`GameplayStatics.SaveGameToSlot` (`self.SG_LevelStates`) _returnvalue)
  (if true
    (`KismetSystemLibrary.PrintText` "LevelStates Saved to save game file" true true (struct :`R` 0.06892 :`G` 1.0 :`A` 1.0) 5.0)
    (else
      (`KismetSystemLibrary.PrintText` "LevelStates  FAILED TO SAVE" true true (struct :`R` 1.0 :`B` 0.001431 :`A` 1.0) 5.0))))

(event `LoadLevelState`
  (bind _returnvalue (`GameplayStatics.GetCurrentLevelName` true))
  (bind _returnvalue_2 (`GameplayStatics.DoesSaveGameExist` _returnvalue))
  (if _returnvalue_2
    (bind _returnvalue_3 (`GameplayStatics.LoadGameFromSlot` _returnvalue))
    (bind _assg_level_states (cast `/Game/Blueprints/Coding2Blueprints/SavingLoading/SG_LevelStates` _returnvalue_3))
    (bind _output_get (set `self.SG_LevelStates` _assg_level_states))
    (`self.UpdateLevelInfo` _output_get)
    (else
      (bind _returnvalue_4 (`GameplayStatics.CreateSaveGameObject` "/Game/Blueprints/Coding2Blueprints/SavingLoading/SG_LevelStates.SG_LevelStates_C"))
      (set `self.SG_LevelStates` _returnvalue_4))))

(fn `UpdateLevelInfo`
  (params (LevelStates :type "/Game/Blueprints/Coding2Blueprints/SavingLoading/SG_LevelStates Object Reference"))
  (for _array_element (`/Game/Blueprints/Coding2Blueprints/SavingLoading/SG_LevelStates.CollectedCoins` LevelStates)
    (`/Engine/EditorBlueprintResources/StandardMacros.IsValid` _array_element
      (:`Is Valid`
        (`/Game/Blueprints/Coding2Blueprints/BP_Coin.AlreadyCollected` _array_element))))
  (for _array_element_2 (`/Game/Blueprints/Coding2Blueprints/SavingLoading/SG_LevelStates.KeyDoorOpen` LevelStates)
    (`/Engine/EditorBlueprintResources/StandardMacros.IsValid` _array_element_2
      (:`Is Valid`
        (`/Game/Blueprints/Coding2Blueprints/BP_Door.AlreadyOpened` _array_element_2))))
  (for _array_element_3 (`/Game/Blueprints/Coding2Blueprints/SavingLoading/SG_LevelStates.CameraDoorOpen` LevelStates)
    (`/Engine/EditorBlueprintResources/StandardMacros.IsValid` _array_element_3)))

(fn `UpdatePlayerInfo1`
  (params (NewParam :type "/Game/Blueprints/Coding2Blueprints/SavingLoading/SG_PlayerStats Object Reference"))
  (bind _asbp_third_person_character (cast `/Game/ThirdPerson/Blueprints/BP_ThirdPersonCharacter` (`GameplayStatics.GetPlayerCharacter` 0)))
  (set `/Game/ThirdPerson/Blueprints/BP_ThirdPersonCharacter.Stamina` (`/Game/Blueprints/Coding2Blueprints/SavingLoading/SG_PlayerStats.Stamina` NewParam) _asbp_third_person_character) ; needs to come out of the charecter
  (set `/Game/ThirdPerson/Blueprints/BP_ThirdPersonCharacter.Health` (`/Game/Blueprints/Coding2Blueprints/SavingLoading/SG_PlayerStats.Health` NewParam) _asbp_third_person_character)
  (set `/Game/ThirdPerson/Blueprints/BP_ThirdPersonCharacter.Mana` (`/Game/Blueprints/Coding2Blueprints/SavingLoading/SG_PlayerStats.Mana` NewParam) _asbp_third_person_character))

(fn `UserConstructionScript`)