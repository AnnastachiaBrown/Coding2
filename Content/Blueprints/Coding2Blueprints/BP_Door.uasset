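; BP_Door is a key-locked door that slides down when the third-person character overlaps its collision while holding at least one key.
; Opening adds the door to the game mode's GM_SaveLoad level state and plays a timeline that lerps the door mesh's relative Z, without consuming a key.
; A separate AlreadyOpened event plays the same timeline without the key check, and debug strings report door status.
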(event `AlreadyOpened`
  (bind (_direction _newtrack_0) (`Timeline|DoorMov` :!label _label)
    (:`Update`
      (`SceneComponent.K2_SetRelativeLocation` (`self.door`) (`KismetMathLibrary.MakeVector` 0.0 0.0 (`KismetMathLibrary.Lerp` 140.0 -130.0 _newtrack_0)) false false))))

(event `self.ReceiveBeginPlay`
  (`KismetSystemLibrary.PrintString` "Door Exist" true true (struct :`R` 0.229185 :`G` 1.0 :`A` 1.0)))

(event `self.Collision.OnComponentBeginOverlap`
  (params (OverlappedComponent :type "PrimitiveComponent Object Reference") (OtherActor :type "Actor Object Reference") (OtherComp :type "PrimitiveComponent Object Reference") (OtherBodyIndex :type Integer) (bFromSweep :type Boolean) (SweepResult :type "HitResult Structure (by ref)"))
  (bind _asbp_third_person_character (cast `/Game/ThirdPerson/Blueprints/BP_ThirdPersonCharacter` OtherActor))
  (if (> (`/Game/ThirdPerson/Blueprints/BP_ThirdPersonCharacter.KeyTotal` _asbp_third_person_character) 0)
    (`KismetSystemLibrary.PrintString` "Player Open Door" true true (struct :`R` 0.229185 :`G` 1.0 :`A` 1.0))
    (bind _asgm_save_load (cast `/Game/Blueprints/Coding2Blueprints/SavingLoading/GM_SaveLoad` (`GameplayStatics.GetGameMode`)))
    (`KismetArrayLibrary.Array_AddUnique` (`/Game/Blueprints/Coding2Blueprints/SavingLoading/SG_LevelStates.KeyDoorOpen` (`/Game/Blueprints/Coding2Blueprints/SavingLoading/GM_SaveLoad.SG_LevelStates` _asgm_save_load)) self)
    (goto _label)
    (else
      (`KismetSystemLibrary.PrintString` "need KEY" true true (struct :`R` 1.0 :`B` 0.055785 :`A` 1.0)))))

(fn `UserConstructionScript`)