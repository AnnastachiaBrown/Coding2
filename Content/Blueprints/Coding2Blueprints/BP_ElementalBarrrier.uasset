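; BP_ElementalBarrrier is an elemental barrier that kills a player lacking the matching immunity.
; On BeginPlay it writes its Element enum name into two text labels.
; When a BP_ThirdPersonCharacter overlaps the Barier component with an ElementalImmunity different from Element, it prints a red death message and quits the game after a short delay.
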(event `self.ReceiveBeginPlay`
  (bind _returnvalue (`KismetTextLibrary.Conv_StringToText` (`KismetStringLibrary.Concat_StrStr` "barrier of " (`|GetEnumeratorNameAsString` (`self.Element`)))))
  (`KismetSystemLibrary.PrintString` "Barrier Exist" true true (struct :`R` 0.657476 :`G` 1.0 :`A` 1.0))
  (`TextRenderComponent.K2_SetText` (`self.ElementalType`) _returnvalue)
  (`TextRenderComponent.K2_SetText` (`self.ElementalType1`) _returnvalue))

(event `self.Barier.OnComponentBeginOverlap`
  (params (OverlappedComponent :type "PrimitiveComponent Object Reference") (OtherActor :type "Actor Object Reference") (OtherComp :type "PrimitiveComponent Object Reference") (OtherBodyIndex :type Integer) (bFromSweep :type Boolean) (SweepResult :type "HitResult Structure (by ref)"))
  (bind _asbp_third_person_character (cast `/Game/ThirdPerson/Blueprints/BP_ThirdPersonCharacter` OtherActor))
  (if (not (`|EnumEquality` (`/Game/ThirdPerson/Blueprints/BP_ThirdPersonCharacter.ElementalImmunity` _asbp_third_person_character) (`self.Element`)))
    (`KismetSystemLibrary.PrintText` "YOU DEAD" true true (struct :`R` 1.0 :`B` 0.001431 :`A` 1.0))
    (`KismetSystemLibrary.Delay` 1.0)
    (`KismetSystemLibrary.QuitGame` null "Quit")))

(fn `UserConstructionScript`)