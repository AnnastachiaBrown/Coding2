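; Base enemy Blueprint that provides attack, aggro and patrol functions.
; Attack plays a ninja wheel-kick montage and fires AttackFinished whether it completes or is interrupted.
; Aggro events set a flag and swap the mesh to a red material, restoring the material cached at BeginPlay when aggro drops.
; GetNextPatrolPointLocation steps along an assigned route's spline points, reversing at either end to ping-pong, and returns world locations.
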(event `self.ReceiveBeginPlay`
  (set `self.OriginalMaterial` (`PrimitiveComponent.GetMaterial` (`self.Mesh`) 0)))

(event `Attack`
  (`KismetSystemLibrary.PrintString` "Attack Player")
  (`|PlayMontage` (`self.Mesh`) "/Game/CloseCombatAnimSet/Animations/InPlace/Attacks/NinjaWheelKick_Montage.NinjaWheelKick_Montage"
    (:`OnCompleted`
      _)
    (:`OnInterrupted`
      _))
  (`self.AttackFinished`))

(event `GetAggro`
  (set `self.Aggroed` true)
  (`PrimitiveComponent.SetMaterial` (`self.Mesh`) 0 "/AnimationSharing/AnimSharingRed.AnimSharingRed"))

(event `NoAggro`
  (set `self.Aggroed` false)
  (`PrimitiveComponent.SetMaterial` (`self.Mesh`) 0 (`self.OriginalMaterial`)))

(fn `GetNextPatrolPointLocation`
  (returns (Location :type "Vector Structure"))
  (`/Engine/EditorBlueprintResources/StandardMacros.IsValid` (`self.patrolroutes`)
    (:`Is Valid`
      (set `self.PatrolPointIndex` (+ (`self.PatrolPointIndex`) (`self.PatrolRouteDirection`)))
      (if (or (>= (`self.PatrolPointIndex`) (- (`SplineComponent.GetNumberOfSplinePoints` (`/Game/AI_Blueprints/EnemyBAse/BP_PatrolRoute.Spline` (`self.patrolroutes`))) 1)) (<= (`self.PatrolPointIndex`) 0))
        (set `self.PatrolRouteDirection` (* (`self.PatrolRouteDirection`) -1)))
      (return (`SplineComponent.GetLocationAtSplinePoint` (`/Game/AI_Blueprints/EnemyBAse/BP_PatrolRoute.Spline` (`self.patrolroutes`)) (`self.PatrolPointIndex`) "World")))
    (:`Is Not Valid`
      (`KismetSystemLibrary.PrintText` "NOPATROL"))))

(fn `UserConstructionScript`)