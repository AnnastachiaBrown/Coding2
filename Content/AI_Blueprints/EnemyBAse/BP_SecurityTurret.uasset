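; Security turret that tracks a player character inside its detection sphere, with firing left unfinished.
; Sphere overlap stores the BP_ThirdPersonCharacter and starts two looping timers, which are cleared when the character leaves.
; The faster timer turns the Cube toward the player on yaw only, using RInterpTo with an angle offset.
; The slower timer line-traces to the player but does nothing with the result, and RotatingLook is empty.
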(event `self.Sphere.OnComponentEndOverlap`
  (params (OverlappedComponent :type "PrimitiveComponent Object Reference") (OtherActor :type "Actor Object Reference") (OtherComp :type "PrimitiveComponent Object Reference") (OtherBodyIndex :type Integer))
  (`/Engine/EditorBlueprintResources/StandardMacros.IsValid` OtherActor
    (:`Is Valid`
      (cast `/Game/ThirdPerson/Blueprints/BP_ThirdPersonCharacter` OtherActor)
      (`self.Player`
        (:`then`
          (`KismetSystemLibrary.K2_ClearAndInvalidateTimerHandle` (`self.TimerRef`))
          (`KismetSystemLibrary.K2_ClearAndInvalidateTimerHandle` (`self.FireTimer`)))
        (:`else`)))))

(event `self.Sphere.OnComponentBeginOverlap`
  (params (OverlappedComponent :type "PrimitiveComponent Object Reference") (OtherActor :type "Actor Object Reference") (OtherComp :type "PrimitiveComponent Object Reference") (OtherBodyIndex :type Integer) (bFromSweep :type Boolean) (SweepResult :type "HitResult Structure (by ref)"))
  (`/Engine/EditorBlueprintResources/StandardMacros.IsValid` OtherActor
    (:`Is Valid`
      (bind _asbp_third_person_character (cast `/Game/ThirdPerson/Blueprints/BP_ThirdPersonCharacter` OtherActor))
      (set `self.Player` _asbp_third_person_character)
      (`self.TrackTarget`))))

(event `TrackTarget`
  (bind _returnvalue (`KismetSystemLibrary.K2_SetTimerDelegate` (delegate `MoveTurret`) 0.05 true))
  (set `self.TimerRef` _returnvalue)
  (bind _returnvalue_2 (`KismetSystemLibrary.K2_SetTimerDelegate` (delegate `FireTurrent`) 0.3 true true))
  (set `self.FireTimer` _returnvalue_2))

(event `MoveTurret`
  (bind _player (`self.Player`))
  (bind _cube (`self.Cube`))
  (bind (_returnvalue_roll _returnvalue_pitch _returnvalue_yaw) (`KismetMathLibrary.BreakRotator` (`KismetMathLibrary.RInterpTo` (`SceneComponent.RelativeRotation` _cube) (`KismetMathLibrary.FindLookAtRotation` (`self.K2_GetActorLocation` _player) (`self.K2_GetActorLocation`)) (`GameplayStatics.GetWorldDeltaSeconds`) 100.0)))
  (`/Engine/EditorBlueprintResources/StandardMacros.IsValid` _player
    (:`Is Valid`
      (`SceneComponent.K2_SetRelativeRotation` _cube (`KismetMathLibrary.MakeRotator` 0.0 0.0 (+ _returnvalue_yaw 90.0)) false false))))

(event `FireTurrent`
  (bind (_outhit _returnvalue) (`KismetSystemLibrary.LineTraceSingle` (+ (`self.K2_GetActorLocation`) (0.0 0.0 80.0)) (`self.K2_GetActorLocation` (`self.Player`)) "TraceTypeQuery1"))
  (if _returnvalue
    _))

(event `RotatingLook`)

(fn `UserConstructionScript`)